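; Base Blueprint for Periodic Madness resource deposits that reports their depletion to the mod's deposit registry.
; It overrides PlayDepletedEffect to run OnDepositGotEmptied before the parent effect.
; That function derives a name from its own path, between the last slash and the following dot, and logs it with the actor's location.
; It then passes that name to DepositDepleted on the DepositRegistrySubsystem, found through the SubsystemActorManager.
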(event `self.PlayDepletedEffect`
  (params (descriptor :type "FGResourceDescriptor Class Reference"))
  (`self.onDepositGotEmptied`)
  (`parent.PlayDepletedEffect` descriptor))

(fn `onDepositGotEmptied`
  (bind _returnvalue (`KismetSystemLibrary.GetPathName` self))
  (bind _returnvalue_2 (`KismetStringLibrary.FindSubstring` _returnvalue "/" true true))
  (bind _returnvalue_3 (`KismetStringLibrary.GetSubstring` _returnvalue (+ _returnvalue_2 1) (- (- (`KismetStringLibrary.Len` _returnvalue) _returnvalue_2) 1)))
  (bind _returnvalue_4 (`KismetStringLibrary.GetSubstring` _returnvalue_3 0 (`KismetStringLibrary.FindSubstring` _returnvalue_3 "." true)))
  (`BlueprintLoggingLibrary.LogVerbose` (`KismetTextLibrary.Conv_TextToString` (`|FormatText` "{Deposit} at X: {X} Y: {Y} Z: {Z} got depleted." _returnvalue_4 (.x (.location (`self.GetTransform`))) (.y (.location (`self.GetTransform`))) (.z (.location (`self.GetTransform`))))))
  (`/PeriodicMadness/Subsystems/PeriodicMadness_DepositRegistrySubsystem.DepositDepleted` (`SubsystemActorManager.K2_GetSubsystemActor` (subsystem `SubsystemActorManager`) "/PeriodicMadness/Subsystems/PeriodicMadness_DepositRegistrySubsystem.PeriodicMadness_DepositRegistrySubsystem_C") _returnvalue_4)
  (return))

(fn `UserConstructionScript`)