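; Subsystem that removes resource node static mesh actors from the world.
; On BeginPlay, and again whenever a Tick counter reaches its interval, it scans every StaticMeshActor.
; It destroys any whose mesh matches one of a hard-coded set of ore, quartz, sulfur and stone meshes, logging each removal.
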(event `self.ReceiveBeginPlay`
  (`BlueprintLoggingLibrary.LogVerbose` (`KismetTextLibrary.Conv_TextToString` (`|FormatText` "Resource cleaner subsystem initialized.")))
  (`|ExecutionSequence` :!label _label
    (:`then_1`
      (bind _outactors (`GameplayStatics.GetAllActorsOfClass` "/Script/Engine.StaticMeshActor"))
      (for _array_element _outactors
        (bind _staticmesh (`StaticMeshComponent.StaticMesh` (`StaticMeshActor.StaticMeshComponent` _array_element)))
        (if (or (== _staticmesh "/Game/FactoryGame/Resource/RawResources/Nodes/ResourceNode_OreIron_01.ResourceNode_OreIron_01") (== _staticmesh "/Game/FactoryGame/Resource/RawResources/Nodes/ResourceNode_OreCopper_01.ResourceNode_OreCopper_01") (== _staticmesh "/Game/FactoryGame/Resource/RawResources/Nodes/ResourceNode_quartz.ResourceNode_quartz") (== _staticmesh "/Game/FactoryGame/Resource/RawResources/Nodes/ResourceNode_OreGold_01.ResourceNode_OreGold_01") (== _staticmesh "/Game/FactoryGame/Resource/RawResources/Nodes/SulfurResource_01.SulfurResource_01") (== _staticmesh "/Game/FactoryGame/Resource/RawResources/Nodes/Resource_Stone_01.Resource_Stone_01"))
          (`BlueprintLoggingLibrary.LogVerbose` (`KismetTextLibrary.Conv_TextToString` (`|FormatText` "Removing static mesh {StaticMesh}" (`KismetSystemLibrary.GetPathName` _array_element))))
          (`self.K2_DestroyActor` _array_element))))))

(event `self.ReceiveTick`
  (params (DeltaSeconds :type "Float (single-precision)"))
  (bind _output_get (set `self.mCurrentTick` (+ (`self.mCurrentTick`) 1)))
  (if (== _output_get (`self.mTickInterval`))
    (set `self.mCurrentTick` 0)
    (goto _label)))

(fn `UserConstructionScript`)